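; Arcane Shards gameplay ability: shows a magic circle, then on input release targets the ground under the mouse for an area attack.
; A spawned BP_PointsCollection supplies randomly rotated ground points, with the number used set by ability level.
; After the cast montage event and commit, a looping timer triggers shards point by point.
; Each shard fires a GameplayCue and applies radial damage with outward, pitched knockback to nearby live players.
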(event Custom|SpawnShard
  (if (< (Variables|Default|GetCount) (Variables|Default|GetNumsToSpawn))
    (CallFunction|StoreShardSpawnLocation)
    (CallFunction|StoreOverlappingPlayers)
    (for _array_element (Variables|Default|GetPlayersToDamage)
      (CallFunction|RadialDamagetoPlayer _array_element))
    (Math|Integer|IncrementInt (Variables|Default|GetCount)
      (:%20%20
        (Class|GameplayAbility|ExecuteGameplayCuewithParams "(TagName=\"GameplayCue.ArcaneShards\")" (Ability|GameplayCue|MakeGameplayCueParameters :Location (Variables|Default|GetShardSpawnLocation)))))
    (else
      (Utilities|Time|ClearandInvalidateTimerbyHandle (Variables|Default|GetShardSpawnTimer))
      (Actor|DestroyActor (Variables|Default|GetPointsCollection))
      (Ability|EndAbility))))

(event Ability|EventActivateAbility
  (Class|PlayerInterface|ShowMagicCircle(Message) (Ability|GetAvatarActorfromActorInfo) 0)
  (Ability|Tasks|WaitInputRelease false
    (:OnRelease
      (bind _datahandle (|TargetDataUnderMouse)
        (:ValidData
          (Variables|Default|SetMouseHitLocation (.impactpoint (Ability|TargetData|GetHitResultfromTargetData _datahandle)))
          (bind _returnvalue (Game|SpawnActorfromClass "/Game/Blueprints/AbilitySystem/Common/BP_PointsCollection.BP_PointsCollection_C" (Math|Transform|MakeTransform (Variables|Default|GetMouseHitLocation) "0, 0, 0" "1.000000,1.000000,1.000000") "AlwaysSpawn" "MultiplyWithRoot" 0 0))
          (Variables|Default|SetPointsCollection _returnvalue)
          (Variables|Default|SetGroundPoints (Class|PointCollection|GetGroundPoints (Variables|Default|GetPointsCollection) (Variables|Default|GetMouseHitLocation) (Variables|Default|GetMaxNumShards) (Math|Random|RandomFloatinRange 0.0 3.6e+02)))
          (Variables|Default|SetNumsToSpawn (Class|ArcaneShards|GetPointsbyAbilityLevel))
          (Utilities|FlowControl|Sequence
            (:then_0
              (Class|CombatInterface|UpdateFacingTarget(Message) (Ability|GetAvatarActorfromActorInfo) (Variables|Default|GetMouseHitLocation)))
            (:then_1
              ;[1 1 1] Montage
              (|PlayMontageandWaitProxy "None" "/Game/Assets/Characters/Aura/Animations/Abilities/AM_Cast_ArcaneShards.AM_Cast_ArcaneShards" 1.0 "None" false 1.0 0.0 false
                (:then
                  (Ability|Tasks|WaitGameplayEvent "(TagName=\"Event.Montage.ArcaneShards\")" 0 true
                    (:EventReceived
                      (bind _returnvalue_2 (Ability|CommitAbility))
                      (if _returnvalue_2
                        (bind _returnvalue_3 (Utilities|Time|SetTimerbyEvent (delegate Custom|SpawnShard) (Variables|Default|GetShardSpawnDeltaTime) true))
                        (Variables|Default|SetShardSpawnTimer _returnvalue_3)
                        (CallFunction|SpawnShard)
                        (Class|PlayerInterface|HideMagicCircle(Message) (Ability|GetAvatarActorfromActorInfo))
                        (else
                          (Ability|EndAbility))))))))))))))

(fn StoreShardSpawnLocation
  (Variables|Default|SetShardSpawnLocation (Transformation|GetWorldLocation (Utilities|Array|Get(acopy) (Variables|Default|GetGroundPoints) (Variables|Default|GetCount)))))

(fn StoreOverlappingPlayers
  (bind _returnvalue (Ability|GetAvatarActorfromActorInfo))
  (bind _outoverlappingactors (Class|AuraAbilitySystemLibrary|GetLivePlayersWithinRadius _returnvalue (Utilities|Array|MakeArray _returnvalue) (Variables|Default|GetRadialDamageOuterRadius) (Variables|Default|GetShardSpawnLocation)))
  (Variables|Default|SetPlayersToDamage _outoverlappingactors)
  (return))

(fn RadialDamagetoPlayer
  (params (TargetActor :type Actor%20Object%20Reference))
  (bind _returnvalue (Transformation|GetActorLocation TargetActor))
  (bind _shardspawnlocation (Variables|Default|GetShardSpawnLocation))
  (bind _returnvalue_2 (- _returnvalue _shardspawnlocation))
  (Class|AuraAbilitySystemLibrary|ApplyDamageEffect (Class|DamageAbility|MakeDamageEffectParamsfromClassDefaults TargetActor (Variables|Default|GetShardSpawnLocation) true _returnvalue_2 true _returnvalue_2 true 45.0)))