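; Base enemy character Blueprint that supplies the spawn and death-style dissolve visuals and facing support for enemies.
; BeginPlay calls Spawning, followed by a one-second Delay that leads to nothing.
; Four events take a dynamic material instance and play separate body or weapon timelines, for spawning or dissolving, that drive its Dissolve scalar.
; UpdateFacingTarget feeds a location into the MotionWarping "FacingTarget" warp target.
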(event EventBeginPlay
  (Class|AuraCharacterBase|Spawning)
  (Utilities|FlowControl|Delay 1.0))

(event EventTick
  (params (DeltaSeconds :type Float%20%28single-precision%29)))

(event EventStartDissolveTimeline
  (params (DynamicDissolveMaterialInstance :type Material%20Instance%20Dynamic%20Object%20Reference))
  (bind _dissolvetrack (Timeline|DissolveBodyTimeline Play)
    (:Update
      (Rendering|Material|SetScalarParameterValue DynamicDissolveMaterialInstance "Dissolve" _dissolvetrack :!class /Script/Engine.MaterialInstanceDynamic))))

(event EventStartWeaponDissolveTimeline
  (params (DynamicDissolveMaterialInstance :type Material%20Instance%20Dynamic%20Object%20Reference))
  (bind _dissolvetrack (Timeline|DissolveWeaponTimeline Play)
    (:Update
      (Rendering|Material|SetScalarParameterValue DynamicDissolveMaterialInstance "Dissolve" _dissolvetrack :!class /Script/Engine.MaterialInstanceDynamic))))

(event EventUpdateFacingTarget
  (params (TargetLocation :type Vector%20%28by%20ref%29 :default "0, 0, 0"))
  (Class|MotionWarpingComponent|AddorUpdateWarpTargetfromLocation (Variables|Default|GetMotionWarping) "FacingTarget" TargetLocation))

(event EventStartWeaponSpawningTimeline
  (params (DynamicDissolveMaterialInstance :type Material%20Instance%20Dynamic%20Object%20Reference))
  (bind _dissolvetrack (Timeline|SpawningWeapoin%20Timeline Play)
    (:Update
      (Rendering|Material|SetScalarParameterValue DynamicDissolveMaterialInstance "Dissolve" _dissolvetrack :!class /Script/Engine.MaterialInstanceDynamic))))

(event EventStartSpawningTimeline
  (params (DynamicDissolveMaterialInstance :type Material%20Instance%20Dynamic%20Object%20Reference))
  (bind _dissolvetrack (Timeline|SpawningBodyTimeline Play)
    (:Update
      (Rendering|Material|SetScalarParameterValue DynamicDissolveMaterialInstance "Dissolve" _dissolvetrack :!class /Script/Engine.MaterialInstanceDynamic))))

(fn ConstructionScript)