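; Base actor whose mesh can fade out and back in through a timeline-driven "Fade" material parameter.
; Construction caches the original materials and builds dynamic instances from the fade materials.
; FadeOut swaps those in and plays the timeline, while Fadein reverses it.
; On finish, a value of 1 restores the originals, and BlockVisibility optionally toggles Visibility-channel collision to Block at 1 or Ignore at 0.
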(event EventBeginPlay)

(event EventFadeOut
  (CallFunction|SetMaterialstoDynamicInstances)
  (bind _fade (Timeline|FadeTimeline Play)
    (:Update
      (for _array_element (Variables|Default|GetDynamicMaterialInstance)
        (Rendering|Material|SetScalarParameterValue _array_element "Fade" _fade :!class /Script/Engine.MaterialInstanceDynamic)))
    (:Finished
      (CallFunction|FadeFinish _fade))))

(event EventFadein
  (bind _fade (Timeline|FadeTimeline Reverse)
    (:Update
      (for _array_element (Variables|Default|GetDynamicMaterialInstance)
        (Rendering|Material|SetScalarParameterValue _array_element "Fade" _fade :!class /Script/Engine.MaterialInstanceDynamic)))
    (:Finished
      (CallFunction|FadeFinish _fade))))

(fn ConstructionScript
  (Utilities|Array|Clear (Variables|Default|GetDynamicMaterialInstance))
  (Variables|Default|SetOriginalMaterials (Rendering|Material|GetMaterials (Variables|Default|GetMesh)))
  (for _array_element (Variables|Default|GetFadeMatericalInstances)
    (bind _returnvalue (Rendering|Material|CreateDynamicMaterialInstance _array_element "None" "None" :!class /Script/Engine.KismetMaterialLibrary))
    (Utilities|Array|AddUnique (Variables|Default|GetDynamicMaterialInstance) _returnvalue)))

(fn SetMaterialstoDynamicInstances
  (for (_array_element _array_index) (Variables|Default|GetDynamicMaterialInstance)
    (Rendering|Material|SetMaterial (Variables|Default|GetMesh) _array_index _array_element)))

(fn ResetMaterial
  (for (_array_element _array_index) (Variables|Default|GetOriginalMaterials)
    (Rendering|Material|SetMaterial (Variables|Default|GetMesh) _array_index _array_element)))

(fn FadeFinish
  (params (Fade :type Float%20%28double-precision%29))
  (if (>= Fade 1.0)
    (CallFunction|ResetMaterial)
    (if (Variables|Default|GetBlockVisibility)
      (Collision|SetCollisionResponsetoChannel (Variables|Default|GetMesh) "ECC_Visibility" "ECR_Block"))
    (elif (<= Fade 0.0)
      (if (Variables|Default|GetBlockVisibility)
        (Collision|SetCollisionResponsetoChannel (Variables|Default|GetMesh) "ECC_Visibility" "ECR_Ignore")))))