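; Fireball ability projectile that flies out along its forward vector, then returns to ReturnToActor and explodes within ExplodeDistance of it.
; StartOutgoingTimeline runs on authority only, chaining two timelines that lerp location without sweeping, with the return leg tracking the target's current position.
; The explosion calls OnHit, applies radial damage effect params to nearby live players (excluding owner) with upward-angled knockback and death impulse, then destroys the actor.
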(event EventStartOutgoingTimeline
  (Networking|SwitchHasAuthority
    (:Authority
      (Variables|Default|SetInitialLocation (Transformation|GetActorLocation))
      (Variables|Default|SetApexLocation (+ (Variables|Default|GetInitialLocation) (* (Transformation|GetActorForwardVector) (Variables|Default|GetTravelDistance))))
      (bind _outgoingtrack (Timeline|OutGoingTimeline Play)
        (:Update
          (Transformation|SetActorLocation (Math|Vector|Lerp(Vector) (Variables|Default|GetInitialLocation) (Variables|Default|GetApexLocation) _outgoingtrack) false false))
        (:Finished
          (bind _returningtrack (Timeline|ReturningTimeline Play)
            (:Update
              (Transformation|SetActorLocation (Math|Vector|Lerp(Vector) (Variables|Default|GetApexLocation) (Transformation|GetActorLocation (Variables|Default|GetReturnToActor)) _returningtrack) false false)
              (if (CallFunction|IsWithinExplodeDistance)
                (Class|AuraProjectile|OnHit)
                (bind _outoverlappingactors (Class|AuraAbilitySystemLibrary|GetLivePlayersWithinRadius self (Utilities|Array|MakeArray (Components|GetOwner) self) 3e+02 (Transformation|GetActorLocation)))
                (Class|AuraAbilitySystemLibrary|SetIsRadialDamageEffectParam (Variables|Default|GetDamageEffectParams) true 3e+01 5e+01 (Transformation|GetActorLocation))
                (for _array_element _outoverlappingactors
                  (Class|AuraAbilitySystemLibrary|SetTargetEffectParamsASC (Variables|Default|GetDamageEffectParams) (Ability|GetAbilitySystemComponent _array_element))
                  (Class|AuraAbilitySystemLibrary|SetKnockbackDirection (Variables|Default|GetDamageEffectParams) (Math|Vector|GetForwardVector (Math|Rotator|MakeRotator (.roll (Math|Rotator|MakeRotfromX (- (Transformation|GetActorLocation _array_element) (Transformation|GetActorLocation)))) 45.0 (.yaw (Math|Rotator|MakeRotfromX (- (Transformation|GetActorLocation _array_element) (Transformation|GetActorLocation)))))) 8e+02)
                  (Class|AuraAbilitySystemLibrary|SetDeathImpulseDirection (Variables|Default|GetDamageEffectParams) (Math|Vector|GetForwardVector (Math|Rotator|MakeRotator (.roll (Math|Rotator|MakeRotfromX (- (Transformation|GetActorLocation _array_element) (Transformation|GetActorLocation)))) 45.0 (.yaw (Math|Rotator|MakeRotfromX (- (Transformation|GetActorLocation _array_element) (Transformation|GetActorLocation)))))) 8e+02)
                  (Class|AuraAbilitySystemLibrary|ApplyDamageEffect (Variables|Default|GetDamageEffectParams)))
                (Actor|DestroyActor)))))))))

(fn ConstructionScript)

(fn IsWithinExplodeDistance
  (return (<= (Math|Vector|VectorLength (- (Transformation|GetActorLocation) (Transformation|GetActorLocation (Variables|Default|GetReturnToActor)))) (Variables|Default|GetExplodeDistance))))